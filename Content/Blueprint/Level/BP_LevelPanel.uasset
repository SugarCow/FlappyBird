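; BP_LevelPanel is a moving level segment that carries a pipe pair, apparently for a Flappy Bird-style scroller.
; BeginPlay randomizes the gap between two middle markers, then spawns a BP_Pipe at each with a shared random vertical shift, rotating the upper sprite.
; Tick moves the panel along local X by PanelSpeed, and CheckAndDeletePanel destroys it once player X plus panel X falls below a threshold.
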(event EventBeginPlay
  (bind _bottommiddle (Variables|Default|GetBottomMiddle))
  (bind _uppermiddle (Variables|Default|GetUpperMiddle))
  (bind _bottommiddle_2 (Variables|Default|GetBottomMiddle))
  (bind _uppermiddle_2 (Variables|Default|GetUpperMiddle))
  (bind _returnvalue (Transformation|GetWorldLocation _bottommiddle))
  (bind _returnvalue_2 (Transformation|GetWorldLocation _uppermiddle_2))
  (bind _output_get (Variables|Default|SetOffset (Math|Random|RandomFloatinRange 55.0 9e+01)))
  (Utilities|FlowControl|Sequence
    (:then_0
      (Transformation|SetRelativeLocation _bottommiddle_2 (- (Variables|/Script/Engine.SceneComponent|GetRelativeLocation _bottommiddle_2) (Math|Vector|MakeVector 0.0 0.0 _output_get)) false false))
    (:then_1
      (Transformation|SetRelativeLocation _uppermiddle (+ (Variables|/Script/Engine.SceneComponent|GetRelativeLocation _uppermiddle) (Math|Vector|MakeVector 0.0 0.0 _output_get)) false false)
      (Utilities|FlowControl|Sequence
        (:then_0
          (Variables|Default|SetOffset (Math|Random|RandomFloatinRange -2.2e+02 2.2e+02))
          (bind _returnvalue_3 (Game|SpawnActorfromClass "/Game/Blueprint/Level/BP_Pipe.BP_Pipe_C" (Math|Transform|MakeTransform (Math|Vector|MakeVector (.x _returnvalue_2) (.y _returnvalue_2) (- (.z _returnvalue_2) (Variables|Default|GetOffset))) "0, 0, 0" "1.000000,1.000000,1.000000") "Undefined" "MultiplyWithRoot" 0 0))
          (Transformation|SetRelativeRotation (Variables|/Game/Blueprint/Level/BP_Pipe.BP_Pipe_C|GetPipe_Sprite _returnvalue_3) "180.000000,0.000000,0.000000" false false))
        (:then_1
          (Game|SpawnActorfromClass "/Game/Blueprint/Level/BP_Pipe.BP_Pipe_C" (Math|Transform|MakeTransform (Math|Vector|MakeVector (.x _returnvalue) (.y _returnvalue) (- (.z _returnvalue) (Variables|Default|GetOffset))) "0, 0, 0" "1.000000,1.000000,1.000000") "Undefined" "MultiplyWithRoot" 0 0)
          (Development|PrintString "pipespawned"))))))

(event EventTick
  (params (DeltaSeconds :type Float%20%28single-precision%29))
  (Transformation|AddActorLocalOffset (Math|Vector|MakeVector (* DeltaSeconds (Variables|Default|GetPanelSpeed)) 0.0 0.0) false false)
  (CallFunction|CheckandDeletePanel))

(fn ConstructionScript)

(fn CheckandDeletePanel
  (if (< (+ (.x (Transformation|GetActorLocation (Game|GetPlayerCharacter 0))) (.x (Transformation|GetActorLocation self))) -1e+03)
    (Development|PrintString "destryoed")
    (Actor|DestroyActor)))