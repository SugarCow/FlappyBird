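; Pipe obstacle actor that moves continuously and awards a point to the player on passing through its trigger.
; Tick offsets the actor along its local X axis by PipeSpeed scaled by delta time, without sweeping.
; When BP_Player overlaps PointTrigger, the pipe increments that player's Point and prints the total.
; BeginPlay checks IsBottomPipe, but the branch does nothing.
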(event OnComponentBeginOverlap(PointTrigger)
  (params (OverlappedComponent :type Primitive%20Component%20Object%20Reference) (OtherActor :type Actor%20Object%20Reference) (OtherComp :type Primitive%20Component%20Object%20Reference) (OtherBodyIndex :type Integer) (bFromSweep :type Boolean) (SweepResult :type Hit%20Result%20Structure%20%28by%20ref%29))
  (bind _asbp_player (Utilities|Casting|CastToBP_Player OtherActor))
  (bind _result (Math|Integer|IncrementInt (Variables|/Game/Blueprint/Player/BP_Player.BP_Player_C|GetPoint _asbp_player))
    (:%20%20
      (bind _output_get (Variables|/Game/Blueprint/Player/BP_Player.BP_Player_C|SetPoint _asbp_player _result))
      (Development|PrintString (Utilities|String|ToString(Integer) _output_get)))))

(event EventBeginPlay
  (if (Variables|Default|GetIsBottomPipe)
    _))

(event Collision|EventActorBeginOverlap
  (params (OtherActor :type Actor%20Object%20Reference)))

(event EventTick
  (params (DeltaSeconds :type Float%20%28single-precision%29))
  (Transformation|AddActorLocalOffset (Math|Vector|MakeVector (* DeltaSeconds (Variables|Default|GetPipeSpeed)) 0.0 0.0) false false))

(fn ConstructionScript)