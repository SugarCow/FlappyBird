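; BP_PanelSpawner builds the scrolling or endless level by chaining BP_LevelPanel actors, each spawned at the previous panel's NextPannel point.
; At BeginPlay it lays a starting row, flagged as initial outside the Menu level, with pipes on all but the first.
; Outside menu mode, a looping timer keeps appending panels with pipes.
; The Menu level gets a pipe-free row plus MenuPanelSpawning, a DoOnce-throttled spawn that leaves CurrentPanel unchanged.
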(event Custom|MenuPanelSpawning
  (Utilities|FlowControl|DoOnce false :!label _label
    (:Completed
      (Game|SpawnActorfromClass "/Game/Blueprint/Level/BP_LevelPanel.BP_LevelPanel_C" (Math|Transform|MakeTransform (Transformation|GetWorldLocation (Variables|/Game/Blueprint/Level/BP_LevelPanel.BP_LevelPanel_C|GetNextPannel (Variables|Default|GetCurrentPanel))) "0, 0, 0" "6.000000,6.000000,6.000000") "Undefined" "MultiplyWithRoot" 0 0)
      (Utilities|FlowControl|Delay 2.0)
      (goto _label Reset))))

(event EventBeginPlay
  (bind _asgm_game_mode (Utilities|Casting|CastToGM_GameMode (Game|GetGameMode)))
  (if (Variables|/Game/Blueprint/GM_GameMode.GM_GameMode_C|GetIsMenu? _asgm_game_mode)
    (CallFunction|SpawnInitialPanels)
    (else
      (CallFunction|SpawnInitialPanels)
      (CallFunction|SpawnPanel)
      (Utilities|Time|SetTimerbyFunctionName 0 "SpawnPanel" 2.5 true))))

(event Collision|EventActorBeginOverlap
  (params (OtherActor :type Actor%20Object%20Reference)))

(event EventTick
  (params (DeltaSeconds :type Float%20%28single-precision%29)))

(fn ConstructionScript)

(fn SpawnPanel
  (bind _returnvalue (Game|SpawnActorfromClass "/Game/Blueprint/Level/BP_LevelPanel.BP_LevelPanel_C" (Math|Transform|MakeTransform (Transformation|GetWorldLocation (Variables|/Game/Blueprint/Level/BP_LevelPanel.BP_LevelPanel_C|GetNextPannel (Variables|Default|GetCurrentPanel))) "0, 0, 0" "6.000000,6.000000,6.000000") "Undefined" "MultiplyWithRoot" 0 0))
  (bind _output_get (Variables|Default|SetCurrentPanel _returnvalue))
  (Default|CreatePipes _output_get))

(fn SpawnInitialPanels
  (bind _returnvalue (Game|GetCurrentLevelName true))
  (if (Utilities|Enum|Equal(Enum) _returnvalue "Menu")
    (bind _returnvalue_2 (Game|SpawnActorfromClass "/Game/Blueprint/Level/BP_LevelPanel.BP_LevelPanel_C" (Math|Transform|MakeTransform (Transformation|GetActorLocation) "0, 0, 0" "6.000000,6.000000,6.000000") "Undefined" "MultiplyWithRoot" 0 0))
    (Variables|Default|SetCurrentPanel _returnvalue_2)
    (for _index (range 0 3)
      (bind _returnvalue_3 (Game|SpawnActorfromClass "/Game/Blueprint/Level/BP_LevelPanel.BP_LevelPanel_C" (Math|Transform|MakeTransform (Transformation|GetWorldLocation (Variables|/Game/Blueprint/Level/BP_LevelPanel.BP_LevelPanel_C|GetNextPannel (Variables|Default|GetCurrentPanel))) "0, 0, 0" "6.000000,6.000000,6.000000") "Undefined" "MultiplyWithRoot" 0 0))
      (Variables|Default|SetCurrentPanel _returnvalue_3))
    (CallFunction|MenuPanelSpawning)
    (else
      (bind _returnvalue_4 (Game|SpawnActorfromClass "/Game/Blueprint/Level/BP_LevelPanel.BP_LevelPanel_C" (Math|Transform|MakeTransform (Transformation|GetActorLocation) "0, 0, 0" "6.000000,6.000000,6.000000") "Undefined" "MultiplyWithRoot" 0 0))
      (bind _output_get (Variables|Default|SetCurrentPanel _returnvalue_4))
      (Variables|/Game/Blueprint/Level/BP_LevelPanel.BP_LevelPanel_C|SetInitialPanel? _output_get true)
      (for _index_2 (range 0 1)
        (bind _returnvalue_5 (Game|SpawnActorfromClass "/Game/Blueprint/Level/BP_LevelPanel.BP_LevelPanel_C" (Math|Transform|MakeTransform (Transformation|GetWorldLocation (Variables|/Game/Blueprint/Level/BP_LevelPanel.BP_LevelPanel_C|GetNextPannel (Variables|Default|GetCurrentPanel))) "0, 0, 0" "6.000000,6.000000,6.000000") "Undefined" "MultiplyWithRoot" 0 0))
        (bind _output_get_2 (Variables|Default|SetCurrentPanel _returnvalue_5))
        (Variables|/Game/Blueprint/Level/BP_LevelPanel.BP_LevelPanel_C|SetInitialPanel? _output_get_2 true)
        (Default|CreatePipes _output_get_2)))))